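; Popper is a button-triggered machine that spins a cube and affects Bp_PQ actors touching its Popper component.
; BeginPlay registers ButtonPress with the first-person character, and a matching button sets IsActive false, which is the running state despite the name.
; While running, Tick rotates the cube and a 20-second Delay restores IsActive.
; Overlaps during that window fire Niagara, lower Peckish, and raise Passion and Pep.
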(event OnComponentBeginOverlap(Popper)
  (params (OverlappedComponent :type Primitive%20Component%20Object%20Reference) (OtherActor :type Actor%20Object%20Reference) (OtherComp :type Primitive%20Component%20Object%20Reference) (OtherBodyIndex :type Integer) (bFromSweep :type Boolean) (SweepResult :type Hit%20Result%20Structure%20%28by%20ref%29))
  (if (not (Variables|Default|GetisActive))
    (bind _asbp_pq (Utilities|Casting|CastToBp_PQ OtherActor))
    (Components|Activation|Activate (Variables|Default|GetNiagara) true)
    (Default|ChangePeckish _asbp_pq -3)
    (Variables|/Game/Blueprints/Bp_PQ.Bp_PQ_C|SetPassion _asbp_pq (+ (Variables|/Game/Blueprints/Bp_PQ.Bp_PQ_C|GetPassion _asbp_pq) (Variables|Default|GetPassionINcrease)))
    (Default|ChangePep _asbp_pq 3)))

(event Custom|ButtonPress
  (params (HitButton :type Static%20Mesh%20Component%20Object%20Reference))
  (if (== HitButton (Variables|Default|GetBp_Button))
    (Variables|Default|SetisActive false)))

(event EventBeginPlay
  (bind _asbp_first_person_character (Utilities|Casting|CastToBP_FirstPersonCharacter (Game|GetPlayerCharacter 0)))
  (EventDispatchers|AssignButtonEvent _asbp_first_person_character (delegate Custom|ButtonPress)))

(event Collision|EventActorBeginOverlap
  (params (OtherActor :type Actor%20Object%20Reference)))

(event EventTick
  (params (DeltaSeconds :type Float%20%28single-precision%29))
  (if (not (Variables|Default|GetisActive))
    (CallFunction|Rotate DeltaSeconds)
    (Utilities|FlowControl|Delay 2e+01)
    (Variables|Default|SetisActive true)))

(fn ConstructionScript)

(fn Rotate
  (params (DeltaTime :type Float%20%28double-precision%29))
  (bind _cube (Variables|Default|GetCube))
  (bind _relativerotation (Variables|/Script/Engine.SceneComponent|GetRelativeRotation _cube))
  (Transformation|AddLocalRotation _cube (Math|Rotator|MakeRotator (.roll _relativerotation) (.pitch _relativerotation) (* (Variables|Default|GetRotation) DeltaTime)) false false))