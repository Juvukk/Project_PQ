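; Painter station where the player picks a colour and texture and applies them to a Bp_PQ standing in its collision zone.
; Button events bound through the first-person character cycle wrapping colour and texture indices, previewed on a ColourSelection widget.
; The apply button puts a tinted, textured dynamic material instance on the tracked PQ.
; Tick turns the cylinder toward the player and disables roaming on the tracked PQ while it is unleashed.
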(event OnComponentBeginOverlap(FatherCol)
  (params (OverlappedComponent :type Primitive%20Component%20Object%20Reference) (OtherActor :type Actor%20Object%20Reference) (OtherComp :type Primitive%20Component%20Object%20Reference) (OtherBodyIndex :type Integer) (bFromSweep :type Boolean) (SweepResult :type Hit%20Result%20Structure%20%28by%20ref%29))
  (bind _asbp_pq (Utilities|Casting|CastToBp_PQ OtherActor))
  (Variables|Default|SetPq _asbp_pq))

(event OnComponentEndOverlap(FatherCol)
  (params (OverlappedComponent :type Primitive%20Component%20Object%20Reference) (OtherActor :type Actor%20Object%20Reference) (OtherComp :type Primitive%20Component%20Object%20Reference) (OtherBodyIndex :type Integer))
  (Utilities|Casting|CastToBp_PQ OtherActor)
  (Variables|Default|SetPq 0))

(event Custom|SetPQMaterial
  (params (HitButton :type Static%20Mesh%20Component%20Object%20Reference))
  (bind _pq (Variables|Default|GetPq))
  (if (== HitButton (Variables|Default|GetBp_Button1))
    (if (Utilities|IsValid _pq)
      (CallFunction|SetMaterial _pq)
      (else
        (Development|PrintString "no change Colour")))))

(event EventBeginPlay
  (bind _returnvalue (Game|GetPlayerCharacter 0))
  (|ColourSelectEvents _returnvalue)
  (|TextureSelectEvents _returnvalue)
  (bind _asbp_first_person_character (Utilities|Casting|CastToBP_FirstPersonCharacter _returnvalue))
  (EventDispatchers|AssignButtonEvent _asbp_first_person_character (delegate Custom|SetPQMaterial)))

(event EventTick
  (params (DeltaSeconds :type Float%20%28single-precision%29))
  (bind _cylinder (Variables|Default|GetCylinder))
  (bind _pq (Variables|Default|GetPq))
  (CallFunction|RotateTowardsPlayer _cylinder (Transformation|GetWorldLocation _cylinder) (Transformation|GetActorLocation (Game|GetPlayerCharacter 0)))
  (Utilities|IsValid _pq
    (:Is%20Valid
      (bind _returnvalue (CallFunction|CheckifLeashed _pq))
      (if (not _returnvalue)
        (CallFunction|SetRoam _pq false)))))

(fn ConstructionScript)

(fn ValidateParent
  (params (ParentCollision :type Bp%20PQ%20Object%20Reference)))

(fn SetMaterial
  (params (ActorToSet :type Bp%20PQ%20Object%20Reference))
  (bind _pq_mesh (Variables|/Game/Blueprints/Bp_PQ.Bp_PQ_C|GetPQ_Mesh ActorToSet))
  (bind _returnvalue (Rendering|Material|CreateDynamicMaterialInstance _pq_mesh 0 "/Game/Assets/Materials/Master/Mat_PQMaster.Mat_PQMaster" "None" :!class /Script/Engine.PrimitiveComponent))
  (Rendering|Material|SetTextureParameterValue _returnvalue "Tex" (Variables|Default|GetTexToSet))
  (Rendering|Material|SetVectorParameterValue _returnvalue "Tint" (Variables|Default|GetColourToSet) :!class /Script/Engine.MaterialInstanceDynamic)
  (Rendering|Material|SetMaterial _pq_mesh 0 _returnvalue))

(fn SetRoam
  (params (Parent :type Bp%20PQ%20Object%20Reference) (AllowRoam :type Boolean))
  (if (Utilities|IsValid Parent)
    (if AllowRoam
      (Variables|/Game/Blueprints/Bp_PQ.Bp_PQ_C|SetAiDo Parent "NewEnumerator1")
      (else
        (Variables|/Game/Blueprints/Bp_PQ.Bp_PQ_C|SetAiDo Parent "NewEnumerator3")))))

(fn CheckifLeashed
  (params (Parent :type Bp%20PQ%20Object%20Reference))
  (if (Utilities|IsValid Parent)
    (return (Utilities|Enum|Equal(Enum) (Variables|/Game/Blueprints/Bp_PQ.Bp_PQ_C|GetAiDo Parent) "NewEnumerator0"))))

(fn RotateTowardsPlayer
  (params (Object%20To%20Rotate :type Scene%20Component%20Object%20Reference) (Start :type Vector%20%28by%20ref%29) (Target :type Vector%20%28by%20ref%29))
  (bind _returnvalue (Math|Rotator|FindLookatRotation Start Target))
  (bind _returnvalue_2 (Transformation|GetWorldRotation Object%20To%20Rotate))
  (Transformation|SetWorldRotation Object%20To%20Rotate (Math|Rotator|Lerp(Rotator) (Math|Rotator|MakeRotator (.roll _returnvalue_2) (.pitch _returnvalue_2) (.yaw _returnvalue_2)) (Math|Rotator|MakeRotator (.roll _returnvalue) (.pitch _returnvalue_2) (.yaw _returnvalue)) 1.0 true) false false))

(fn WrapInputforCol
  (params (TooLong :type Boolean) (TooShort :type Boolean) (ArrayLength :type Integer))
  (Utilities|FlowControl|Sequence
    (:then_0
      (if TooLong
        (Variables|Default|SetColourIndex 0)))
    (:then_1
      (if TooShort
        (Variables|Default|SetColourIndex (- ArrayLength 1))))))

(fn ChangeIndex
  (params (Index :type Integer) (ChangeAmount :type Integer))
  (Variables|Default|SetColourIndex (+ Index ChangeAmount)))

(fn ChangeUICol
  (bind _colourindex (Variables|Default|GetColourIndex))
  (bind _allcolours (Variables|Default|GetAllColours))
  (bind _output (Utilities|Array|Get(acopy) _allcolours _colourindex))
  (Utilities|Casting|CastToColourSelection (UserInterface|GetWidget (Variables|Default|GetColourSelection)))
  (Variables|Default|SetColourToSet _output)
  (Class|WidgetComponent|SetTintColorandOpacity (Variables|Default|GetColourSelection) _output))

(fn ChangeUITex
  (bind _texindex (Variables|Default|GetTexIndex))
  (bind _alltextures (Variables|Default|GetAllTextures))
  (bind _output (Utilities|Array|Get(acopy) _alltextures _texindex))
  (bind _ascolour_selection (Utilities|Casting|CastToColourSelection (UserInterface|GetWidget (Variables|Default|GetColourSelection))))
  (Variables|Default|SetTexToSet _output)
  (Default|ChangeTexture _ascolour_selection _output))

(fn WrapInputforTex
  (params (TooLong :type Boolean) (TooShort :type Boolean) (ArrayLength :type Integer))
  (if TooLong
    (Variables|Default|SetTexIndex 0)
    (elif TooShort
      (Variables|Default|SetTexIndex (- ArrayLength 1)))))

(event Custom|TexChangeRight
  (params (HitButton :type Static%20Mesh%20Component%20Object%20Reference))
  (if (== HitButton (Variables|Default|GetRight1))
    (|TextureRightInput)))

(event Custom|TexChangeLeft
  (params (HitButton :type Static%20Mesh%20Component%20Object%20Reference))
  (if (== HitButton (Variables|Default|GetLeft1))
    (|TextureLeftInputCheck)))

(event Custom|UpdateTextUI
  (params (HitButton :type Static%20Mesh%20Component%20Object%20Reference))
  (CallFunction|ChangeUITex))

(event Custom|ColChangeRight
  (params (HitButton :type Static%20Mesh%20Component%20Object%20Reference))
  (if (== HitButton (Variables|Default|GetRight))
    (|ColourRightInputCheck)))

(event Custom|ChangeColourLeft
  (params (HitButton :type Static%20Mesh%20Component%20Object%20Reference))
  (if (== HitButton (Variables|Default|GetLeft))
    (|ColourLeftInputCheck)))

(event Custom|UpdateUI
  (params (HitButton :type Static%20Mesh%20Component%20Object%20Reference))
  (CallFunction|ChangeUICol))