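; Petition station where the player turns in a Bp_PQ creature matching a displayed request to earn money.
; It copies a random existing PQ's traits as requirements and prices them from their sum on a Petition widget, alongside the overlapping PQ's stats.
; Tick halts an unleashed tagged PQ inside MotherCol as the submission.
; Player button events reroll the request or check minimum stats and exact pattern/pigment, then pay out and destroy the PQ.
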(event OnComponentBeginOverlap(MotherCol)
  (params (OverlappedComponent :type Primitive%20Component%20Object%20Reference) (OtherActor :type Actor%20Object%20Reference) (OtherComp :type Primitive%20Component%20Object%20Reference) (OtherBodyIndex :type Integer) (bFromSweep :type Boolean) (SweepResult :type Hit%20Result%20Structure%20%28by%20ref%29))
  (bind _asbp_pq (Utilities|Casting|CastToBp_PQ OtherActor))
  (CallFunction|SetSubmittedText _asbp_pq))

(event OnComponentEndOverlap(MotherCol)
  (params (OverlappedComponent :type Primitive%20Component%20Object%20Reference) (OtherActor :type Actor%20Object%20Reference) (OtherComp :type Primitive%20Component%20Object%20Reference) (OtherBodyIndex :type Integer))
  (bind _asbp_pq (Utilities|Casting|CastToBp_PQ OtherActor))
  (bind _returnvalue (CallFunction|CheckifLeashed _asbp_pq))
  (if (not _returnvalue)
    (CallFunction|SetRoam _asbp_pq true)
    (Variables|Default|SetSubmittedPQ _asbp_pq)))

(event Custom|SubmittPetition
  (params (HitButton :type Static%20Mesh%20Component%20Object%20Reference))
  (if (== HitButton (Variables|Default|GetSubmitButtonn))
    (bind _isvalid (CallFunction|ValidateParent (Variables|Default|GetSubmittedPQ)))
    (if _isvalid
      (bind _valid (CallFunction|CheckSub (Variables|Default|GetSubmittedPQ)))
      (if _valid
        (bind _asbp_first_person_character (Utilities|Casting|CastToBP_FirstPersonCharacter (Game|GetPlayerCharacter 0)))
        (Variables|/Game/Blueprints/BP_FirstPersonCharacter.BP_FirstPersonCharacter_C|SetPlayerMoney _asbp_first_person_character (+ (Variables|/Game/Assets/UI/Petition.Petition_C|GetPriceInt (Variables|Default|GetPetition)) (Variables|/Game/Blueprints/BP_FirstPersonCharacter.BP_FirstPersonCharacter_C|GetPlayerMoney _asbp_first_person_character)))
        (Actor|DestroyActor (Variables|Default|GetSubmittedPQ))))))

(event Custom|RejectButtonEvent
  (params (HitButton :type Static%20Mesh%20Component%20Object%20Reference))
  (if (== HitButton (Variables|Default|GetRejectSubmission))
    (CallFunction|GetPetition)
    (CallFunction|SetRequiredText)))

(event EventBeginPlay
  (bind _asbp_first_person_character (Utilities|Casting|CastToBP_FirstPersonCharacter (Game|GetPlayerCharacter 0)))
  (EventDispatchers|AssignButtonEvent _asbp_first_person_character (delegate Custom|SubmittPetition))
  (|SetPetitionReference)
  (Utilities|FlowControl|Delay 0.2)
  (CallFunction|GetPetition)
  (CallFunction|SetRequiredText)
  (EventDispatchers|AssignButtonEvent _asbp_first_person_character (delegate Custom|RejectButtonEvent)))

(event EventTick
  (params (DeltaSeconds :type Float%20%28single-precision%29))
  (bind _asbp_pq (Utilities|Casting|CastToBp_PQ (Utilities|Array|Get(acopy) (Collision|GetOverlappingActors (Variables|Default|GetMotherCol) "/Game/Blueprints/Bp_PQ.Bp_PQ_C" :!class /Script/Engine.PrimitiveComponent))))
  (bind _returnvalue (CallFunction|CheckifLeashed _asbp_pq))
  (if (not _returnvalue)
    (if (Actor|ActorHasTag _asbp_pq "PQ")
      (bind _output_get (Variables|Default|SetSubmittedPQ _asbp_pq))
      (CallFunction|SetRoam _output_get false)
      (return))))

(fn ConstructionScript)

(fn ValidateParent
  (params (ParentCollision :type Bp%20PQ%20Object%20Reference))
  (bind _returnvalue (Utilities|IsValid ParentCollision))
  (if _returnvalue
    (return ParentCollision _returnvalue)
    (else
      (Development|PrintString (Utilities|String|Append "Parent Invalid:" (Utilities|GetDisplayName ParentCollision))))))

(fn SetRoam
  (params (Parent :type Bp%20PQ%20Object%20Reference) (AllowRoam :type Boolean))
  (if (Utilities|IsValid Parent)
    (if AllowRoam
      (Variables|/Game/Blueprints/Bp_PQ.Bp_PQ_C|SetAiDo Parent "NewEnumerator1")
      (else
        (Variables|/Game/Blueprints/Bp_PQ.Bp_PQ_C|SetAiDo Parent "NewEnumerator3")))))

(fn CheckifLeashed
  (params (Parent :type Bp%20PQ%20Object%20Reference))
  (if (Utilities|IsValid Parent)
    (return (Utilities|Enum|Equal(Enum) (Variables|/Game/Blueprints/Bp_PQ.Bp_PQ_C|GetAiDo Parent) "NewEnumerator0"))))

(fn GetPetition
  (bind _outactors (Actor|GetAllActorsOfClass "/Game/Blueprints/Bp_PQ.Bp_PQ_C"))
  (bind _output_get (Variables|Default|SetRequirePq (Utilities|Array|Get(acopy) _outactors (Math|Random|RandomIntegerinRange 0 (- (Utilities|Array|Length _outactors) -1))) :!label _label))
  (Utilities|IsValid _output_get
    (:Is%20Valid
      (Variables|Default|SetReqPep (Variables|/Game/Blueprints/Bp_PQ.Bp_PQ_C|GetPep _output_get))
      (Variables|Default|SetReqPassion (Variables|/Game/Blueprints/Bp_PQ.Bp_PQ_C|GetPassion _output_get))
      (Variables|Default|SetReqQuality (Variables|/Game/Blueprints/Bp_PQ.Bp_PQ_C|GetQuality _output_get))
      (Variables|Default|SetReqPat (Variables|/Game/Blueprints/Bp_PQ.Bp_PQ_C|GetPassOnTex _output_get))
      (Variables|Default|SetReqPig (Variables|/Game/Blueprints/Bp_PQ.Bp_PQ_C|GetPassOnCol _output_get)))
    (:Is%20Not%20Valid
      (goto _label))))

(fn ToText
  (params (TextToChange :type Text%20Block%20Object%20Reference) (Set :type Integer))
  (Rendering|Components|TextRender|SetText TextToChange (Utilities|Text|ToText(String) (Utilities|String|ToString(Integer) Set))))

(fn SetRequiredText
  (bind _petition (Variables|Default|GetPetition))
  (CallFunction|ToText (Variables|/Game/Assets/UI/Petition.Petition_C|GetRequiredPass _petition) (Variables|Default|GetReqPassion))
  (CallFunction|ToText (Variables|/Game/Assets/UI/Petition.Petition_C|GetRequiredPattern _petition) (Variables|Default|GetReqPat))
  (CallFunction|ToText (Variables|/Game/Assets/UI/Petition.Petition_C|GetRequiredPep _petition) (Variables|Default|GetReqPep))
  (CallFunction|ToText (Variables|/Game/Assets/UI/Petition.Petition_C|GetRequiredPigment _petition) (Variables|Default|GetReqPig))
  (CallFunction|ToText (Variables|/Game/Assets/UI/Petition.Petition_C|GetRequiredQuality _petition) (Variables|Default|GetReqQuality))
  (Variables|/Game/Assets/UI/Petition.Petition_C|SetPriceInt _petition (* (+ (Variables|Default|GetReqQuality) (Variables|Default|GetReqPassion) (Variables|Default|GetReqPep) (Variables|Default|GetReqPat) (Variables|Default|GetReqPig)) 10)))

(fn SetSubmittedText
  (params (Pq :type Bp%20PQ%20Object%20Reference))
  (bind _petition (Variables|Default|GetPetition))
  (CallFunction|ToText (Variables|/Game/Assets/UI/Petition.Petition_C|GetCurrentPass _petition) (Variables|/Game/Blueprints/Bp_PQ.Bp_PQ_C|GetPassion Pq))
  (CallFunction|ToText (Variables|/Game/Assets/UI/Petition.Petition_C|GetCurrentPattern _petition) (Variables|/Game/Blueprints/Bp_PQ.Bp_PQ_C|GetPassOnTex Pq))
  (CallFunction|ToText (Variables|/Game/Assets/UI/Petition.Petition_C|GetCurrentPep _petition) (Variables|/Game/Blueprints/Bp_PQ.Bp_PQ_C|GetPep Pq))
  (CallFunction|ToText (Variables|/Game/Assets/UI/Petition.Petition_C|GetCurrentPigment _petition) (Variables|/Game/Blueprints/Bp_PQ.Bp_PQ_C|GetPassOnCol Pq))
  (CallFunction|ToText (Variables|/Game/Assets/UI/Petition.Petition_C|GetCurrentQual _petition) (Variables|/Game/Blueprints/Bp_PQ.Bp_PQ_C|GetQuality Pq)))

(fn CheckSub
  (params (To%20Check :type Bp%20PQ%20Object%20Reference))
  (Utilities|IsValid To%20Check
    (:Is%20Valid
      (if (>= (Variables|/Game/Blueprints/Bp_PQ.Bp_PQ_C|GetPassion To%20Check) (Variables|Default|GetReqPassion))
        (if (>= (Variables|/Game/Blueprints/Bp_PQ.Bp_PQ_C|GetPep To%20Check) (Variables|Default|GetReqPep))
          (if (>= (Variables|/Game/Blueprints/Bp_PQ.Bp_PQ_C|GetQuality To%20Check) (Variables|Default|GetReqQuality))
            (if (== (Variables|/Game/Blueprints/Bp_PQ.Bp_PQ_C|GetPassOnTex To%20Check) (Variables|Default|GetReqPat))
              (if (== (Variables|/Game/Blueprints/Bp_PQ.Bp_PQ_C|GetPassOnCol To%20Check) (Variables|Default|GetReqPig))
                (LocalVariables|SetAccept? true)
                (else
                  (LocalVariables|SetAccept? false :!label _label)))
              (else
                (goto _label)))
            (else
              (goto _label)))
          (else
            (goto _label)))
        (else
          (goto _label)))
      (return (LocalVariables|GetAccept?)))))