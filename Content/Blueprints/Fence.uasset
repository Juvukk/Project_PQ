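; Fence post actor that links itself to nearby Fence actors with cables and collision.
; On BeginPlay and every Tick, AttachCable sphere-overlaps for other Fences and attaches cable ends to indexed results tagged "Attach".
; It spaces three collision cubes along each link by nested lerps, or returns the cable and first cube to its Cylinder when no neighbor exists.
; GateFence skips the second cable; the search radius is debug-drawn.
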(event EventBeginPlay
  (CallFunction|AttachCable (Variables|Default|GetCable) 1 (Variables|Default|GetCube5) (Variables|Default|GetCube3) (Variables|Default|GetCube4))
  (if (not (Variables|Default|GetGateFence))
    (CallFunction|AttachCable (Variables|Default|GetCable1) 0 (Variables|Default|GetCube) (Variables|Default|GetCube1) (Variables|Default|GetCube2))))

(event Collision|EventActorBeginOverlap
  (params (OtherActor :type Actor%20Object%20Reference)))

(event EventTick
  (params (DeltaSeconds :type Float%20%28single-precision%29))
  (CallFunction|AttachCable (Variables|Default|GetCable) 1 (Variables|Default|GetCube5) (Variables|Default|GetCube3) (Variables|Default|GetCube4))
  (if (not (Variables|Default|GetGateFence))
    (CallFunction|AttachCable (Variables|Default|GetCable1) 0 (Variables|Default|GetCube) (Variables|Default|GetCube1) (Variables|Default|GetCube2))))

(fn ConstructionScript)

(fn AttachCable
  (params (Cable :type Cable%20Component%20Object%20Reference) (ObjectNumber :type Integer) (collision%201 :type Static%20Mesh%20Component%20Object%20Reference) (Collision%202 :type Static%20Mesh%20Component%20Object%20Reference) (Collision%203 :type Static%20Mesh%20Component%20Object%20Reference))
  (bind _returnvalue (Transformation|GetActorLocation))
  (bind _returnvalue_2 (Transformation|GetActorLocation))
  (bind _radius (Variables|Default|GetRadius))
  (bind _cylinder (Variables|Default|GetCylinder))
  (Rendering|Debug|DrawDebugSphere _returnvalue _radius 12 "(R=1.000000,G=1.000000,B=1.000000,A=1.000000)" 0.0)
  (bind _outactors (Collision|SphereOverlapActors _returnvalue _radius (Utilities|Array|MakeArray "ObjectTypeQuery9") "Fence_C" (Utilities|Array|MakeArray self)))
  (Utilities|IsValid (Utilities|Array|Get(acopy) _outactors ObjectNumber)
    (:Is%20Valid
      (if (Actor|ActorHasTag (Utilities|Array|Get(acopy) _outactors ObjectNumber) "Attach")
        (Class|CableComponent|SetAttachEndto Cable (Utilities|Array|Get(acopy) _outactors ObjectNumber) "None" "None")
        (Transformation|SetWorldLocation collision%201 (Math|Vector|Lerp(Vector) _returnvalue_2 (Transformation|GetActorLocation (Utilities|Array|Get(acopy) _outactors ObjectNumber)) 0.5) false true)
        (Transformation|SetWorldLocation Collision%202 (Math|Vector|Lerp(Vector) _returnvalue_2 (Math|Vector|Lerp(Vector) _returnvalue_2 (Transformation|GetActorLocation (Utilities|Array|Get(acopy) _outactors ObjectNumber)) 0.5) 0.5) false true)
        (Transformation|SetWorldLocation Collision%203 (Math|Vector|Lerp(Vector) (Math|Vector|Lerp(Vector) _returnvalue_2 (Transformation|GetActorLocation (Utilities|Array|Get(acopy) _outactors ObjectNumber)) 0.5) (Transformation|GetActorLocation (Utilities|Array|Get(acopy) _outactors ObjectNumber)) 0.5) false true)))
    (:Is%20Not%20Valid
      (Class|CableComponent|SetAttachEndtoComponent Cable _cylinder "None")
      (Transformation|SetWorldLocation collision%201 (Transformation|GetWorldLocation _cylinder) false true))))