(event OnComponentEndOverlap(FatherCol)
  (params (OverlappedComponent :type Primitive%20Component%20Object%20Reference) (OtherActor :type Actor%20Object%20Reference) (OtherComp :type Primitive%20Component%20Object%20Reference) (OtherBodyIndex :type Integer))
  (Variables|Default|SetAllowSpawn true)
  (Rendering|Material|SetMaterial (Variables|Default|GetCube) 0 "/Game/Assets/Materials/Master/Trans.Trans"))

(event OnComponentBeginOverlap(FatherCol)
  (params (OverlappedComponent :type Primitive%20Component%20Object%20Reference) (OtherActor :type Actor%20Object%20Reference) (OtherComp :type Primitive%20Component%20Object%20Reference) (OtherBodyIndex :type Integer) (bFromSweep :type Boolean) (SweepResult :type Hit%20Result%20Structure%20%28by%20ref%29))
  (Variables|Default|SetAllowSpawn false))

(event Custom|SpawnBuilding
  (params (HitButton :type Static%20Mesh%20Component%20Object%20Reference))
  (if (== HitButton (Variables|Default|GetBp_Button1))
    (if (Variables|Default|GetAllowSpawn)
      (bind _output_get (Variables|Default|SetMoneyCheckValue (Variables|/Game/Blueprints/BP_FirstPersonCharacter.BP_FirstPersonCharacter_C|GetPlayerMoney (stale EventBeginPlay _asbp_first_person_character))))
      (if (>= (- _output_get (Math|Conversions|ToInteger(Byte) (Utilities|Array|Get(acopy) (Variables|Default|GetCosts) (Variables|Default|GetTexIndex)))) (Variables|/Game/Blueprints/BP_FirstPersonCharacter.BP_FirstPersonCharacter_C|GetPlayerMoney (stale EventBeginPlay _asbp_first_person_character)))
        (Variables|/Game/Blueprints/BP_FirstPersonCharacter.BP_FirstPersonCharacter_C|SetPlayerMoney (stale EventBeginPlay _asbp_first_person_character) (- _output_get (Math|Conversions|ToInteger(Byte) (Utilities|Array|Get(acopy) (Variables|Default|GetCosts) (Variables|Default|GetTexIndex)))))
        (Game|SpawnActorfromClass (Utilities|Array|Get(acopy) (Variables|Default|GetBuildList) (Variables|Default|GetTexIndex)) (Math|Transform|MakeTransform (.Origin (Collision|GetComponentBounds (Variables|Default|GetFatherCol))) "0, 0, 0" "1.000000,1.000000,1.000000") "Undefined" 0 0)))))

(event EventBeginPlay
  (bind _returnvalue (Game|GetPlayerCharacter 0))
  (|TextureSelectEvents _returnvalue)
  (bind _asbp_first_person_character (Utilities|Casting|CastToBP_FirstPersonCharacter _returnvalue))
  (EventDispatchers|AssignButtonEvent _asbp_first_person_character (delegate Custom|SpawnBuilding))
  (bind _asmoney_ui (Utilities|Casting|CastToMoneyUI (UserInterface|GetWidget (Variables|Default|GetMoneyUI))))
  (Variables|Default|SetAs%20Money%20UI _asmoney_ui))

(event EventTick
  (params (DeltaSeconds :type Float%20%28single-precision%29))
  (CallFunction|ToText (Variables|Default|GetBuildingName) (Variables|Default|GetBuildNames) (Variables|Default|GetTexIndex))
  (CallFunction|ToText (Variables|Default|GetBuildingCost) (Variables|Default|GetCosts) (Variables|Default|GetTexIndex))
  (if (Variables|Default|GetAllowSpawn)
    (CallFunction|ToText (Variables|Default|GetBuildingDesc) (Variables|Default|GetBuildingDes) (Variables|Default|GetTexIndex))
    (Variables|/Game/Assets/UI/MoneyUI.MoneyUI_C|SetMoney (Variables|Default|GetAs%20Money%20UI) (Variables|/Game/Blueprints/BP_FirstPersonCharacter.BP_FirstPersonCharacter_C|GetPlayerMoney (stale EventBeginPlay _asbp_first_person_character)))
    (else
      (Rendering|Components|TextRender|SetText (Variables|Default|GetBuildingDesc) (Utilities|Text|ToText(String) "Bay Blocked"))
      (Rendering|Material|SetMaterial (Variables|Default|GetCube) 0 "/Game/Assets/Materials/Master/Button.Button"))))

(fn ConstructionScript)

(fn RotateTowardsPlayer
  (params (Object%20To%20Rotate :type Scene%20Component%20Object%20Reference) (Start :type Vector%20%28by%20ref%29) (Target :type Vector%20%28by%20ref%29))
  (Transformation|SetWorldRotation Object%20To%20Rotate (Math|Rotator|Lerp(Rotator) (Math|Rotator|MakeRotator (.yaw (Transformation|GetWorldRotation Object%20To%20Rotate)) 0.0 0.0) (Math|Rotator|MakeRotator (.yaw (Math|Rotator|FindLookatRotation Start Target)) 0.0 0.0) 1.0 true) false false))

(fn ChangeUITex
  (bind _texindex (Variables|Default|GetTexIndex))
  (bind _alltextures (Variables|Default|GetAllTextures))
  (bind _output (Utilities|Array|Get(acopy) _alltextures _texindex))
  (bind _ascolour_selection (Utilities|Casting|CastToColourSelection (UserInterface|GetWidget (Variables|Default|GetColourSelection))))
  (Variables|Default|SetTexToSet _output)
  (Default|ChangeTexture _ascolour_selection _output))

(fn WrapInputforTex
  (params (TooLong :type Boolean) (TooShort :type Boolean) (ArrayLength :type Integer))
  (if TooLong
    (Variables|Default|SetTexIndex 0)
    (elif TooShort
      (Variables|Default|SetTexIndex (- ArrayLength 1)))))

(fn ToText
  (params (TextToChange :type Text%20Render%20Component%20Object%20Reference) (StringIN :type Array%20of%20Strings) (Index :type Integer))
  (Rendering|Components|TextRender|SetText TextToChange (Utilities|Text|ToText(String) (Utilities|Array|Get(acopy) StringIN Index))))

(event Custom|TexChangeRight
  (params (HitButton :type Static%20Mesh%20Component%20Object%20Reference))
  (if (== HitButton (Variables|Default|GetRight))
    (|TextureRightInput)))

(event Custom|TexChangeLeft
  (params (HitButton :type Static%20Mesh%20Component%20Object%20Reference))
  (if (== HitButton (Variables|Default|GetLeft))
    (|TextureLeftInputCheck)))

(event Custom|UpdateTextUI
  (params (HitButton :type Static%20Mesh%20Component%20Object%20Reference))
  (CallFunction|ChangeUITex))