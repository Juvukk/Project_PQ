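; Pressable button that the first-person character triggers, sinking briefly and then snapping back to its start position.
; On BeginPlay it registers OpenGate with the character's button event, which flags it pressed when the hit button is itself.
; While it is the player's HitButton, Tick sets the player's looking-at flag and animates the press, resetting after a Delay.
; ValidateButton compares two buttons but is unused in the event graph.
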(event Custom|OpenGate
  (params (HitButton :type Static%20Mesh%20Component%20Object%20Reference))
  (if (== self HitButton)
    (Variables|Default|SetPressed true)))

(event EventBeginPlay
  (bind _asbp_first_person_character (Utilities|Casting|CastToBP_FirstPersonCharacter (Game|GetPlayerCharacter 0)))
  (bind _output_get (Variables|Default|SetPlayer _asbp_first_person_character))
  (EventDispatchers|AssignButtonEvent _output_get (delegate Custom|OpenGate))
  (Variables|Default|SetStartPos (Variables|Default|GetRelativeLocation)))

(event EventTick
  (params (DeltaSeconds :type Float%20%28single-precision%29))
  (bind _player (Variables|Default|GetPlayer))
  (if (== self (Variables|/Game/Blueprints/BP_FirstPersonCharacter.BP_FirstPersonCharacter_C|GetHitButton _player))
    (Variables|/Game/Blueprints/BP_FirstPersonCharacter.BP_FirstPersonCharacter_C|SetIsLookingAtButton _player true)
    (if (Variables|Default|GetPressed)
      (Transformation|AddLocalOffset (Math|Vector|MakeVector 0.0 0.0 (* DeltaSeconds -4e+01)) false false)
      (Utilities|FlowControl|Delay 0.6)
      (Transformation|SetRelativeLocation (Variables|Default|GetStartPos) false false)
      (Variables|Default|SetPressed false))))

(fn ValidateButton
  (params (ButtonOnEvent :type Static%20Mesh%20Component%20Object%20Reference%20%28by%20ref%29) (ButtonOnMachine :type Static%20Mesh%20Component%20Object%20Reference%20%28by%20ref%29))
  (return (== ButtonOnMachine ButtonOnEvent)))