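; Food is an actor with a ProjectileMovement component that destroys itself after LifeTime, using a Delay started from Tick.
; Its GetRandomDirection function gives it an upward launch with a random sideways velocity along either local X or Y, chosen by coin flip.
; The function's call in the event graph is disconnected, so this Blueprint never runs it itself.
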(event EventBeginPlay)

(event EventTick
  (params (DeltaSeconds :type Float%20%28single-precision%29))
  (Utilities|FlowControl|Delay (Variables|Default|GetLifeTime))
  (Actor|DestroyActor))

(fn ConstructionScript)

(fn GetRandomDirection
  (if (Math|Random|RandomBool)
    (Game|Components|ProjectileMovement|SetVelocityinLocalSpace (Variables|Default|GetProjectileMovement) (Math|Vector|MakeVector (Math|Random|RandomFloatinRange -5e+02 5e+02) 0.0 5e+02))
    (else
      (Game|Components|ProjectileMovement|SetVelocityinLocalSpace (Variables|Default|GetProjectileMovement) (Math|Vector|MakeVector 0.0 (Math|Random|RandomFloatinRange -5e+02 5e+02) 5e+02)))))