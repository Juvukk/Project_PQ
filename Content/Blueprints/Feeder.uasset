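; Food dispenser actor that lets the player cycle between animal, vegetable and mineral food and spawn the selected type.
; On BeginPlay it binds switch and dispense handlers to button events from the first-person character.
; Switching advances a wrapping index and updates the FoodUI widget text, while dispensing spawns the matching food at quarter scale at SpawnPoint.
; Tick snaps the cylinder's yaw to face the player.
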(event Custom|ChangeFoodEvent
  (params (HitButton :type Static%20Mesh%20Component%20Object%20Reference))
  (if (== HitButton (Variables|Default|GetSwitchFood))
    (CallFunction|SetFoodIndex)
    (bind _foodget (CallFunction|SelectFood))
    (switch Utilities|FlowControl|Switch|SwitchonFoodType _foodget
      (:NewEnumerator0
        (Variables|Default|SetFoodText "Animal"))
      (:NewEnumerator1
        (Variables|Default|SetFoodText "Vegetables"))
      (:NewEnumerator2
        (Variables|Default|SetFoodText "Minerals")))
    (Rendering|Components|TextRender|SetText (Variables|Default|GetTextReference) (Utilities|Text|ToText(String) (Variables|Default|GetFoodText)))))

(event Custom|DispenceFoodEvent
  (params (HitButton :type Static%20Mesh%20Component%20Object%20Reference))
  (if (== HitButton (Variables|Default|GetDispenseFood))
    (switch Utilities|FlowControl|Switch|SwitchonFoodType (Variables|Default|GetFoodTypes)
      (:NewEnumerator0
        (bind _output_get (CallFunction|GetSpawnLoc))
        (|SpawnAnimal _output_get))
      (:NewEnumerator1
        (bind _output_get_2 (CallFunction|GetSpawnLoc))
        (|SpawnVege _output_get_2))
      (:NewEnumerator2
        (bind _output_get_3 (CallFunction|GetSpawnLoc))
        (|SpawnMineral _output_get_3)))))

(event EventTick
  (params (DeltaSeconds :type Float%20%28single-precision%29))
  (bind _cylinder (Variables|Default|GetCylinder))
  (bind _player (Variables|Default|GetPlayer))
  (Utilities|IsValid _player
    (:Is%20Valid
      (CallFunction|RotateTowardsPlayer _cylinder (Transformation|GetWorldLocation _cylinder) (Transformation|GetActorLocation _player)))))

(event EventBeginPlay
  (bind _player (Variables|Default|GetPlayer))
  (CallFunction|SetPlayerReference)
  (EventDispatchers|AssignButtonEvent _player (delegate Custom|ChangeFoodEvent))
  (EventDispatchers|AssignButtonEvent _player (delegate Custom|DispenceFoodEvent))
  (CallFunction|SelectFood)
  (CallFunction|GetTextReference))

(fn ConstructionScript)

(fn ValidateParent
  (params (ParentCollision :type Bp%20PQ%20Object%20Reference))
  (bind _returnvalue (Utilities|IsValid ParentCollision))
  (if _returnvalue
    (return ParentCollision _returnvalue)
    (else
      (Development|PrintString (Utilities|String|Append "Parent Invalid:" (Utilities|GetDisplayName ParentCollision))))))

(fn SetSpawnerLocation
  (Variables|Default|SetSpawnPos (Transformation|GetWorldTransform (Variables|Default|GetSpawnPoint))))

(fn SetPlayerReference
  (bind _asbp_first_person_character (Utilities|Casting|CastToBP_FirstPersonCharacter (Game|GetPlayerCharacter 0)))
  (Variables|Default|SetPlayer _asbp_first_person_character))

(fn SetFoodIndex
  (if (== (Variables|Default|GetFoodIndex) 2)
    (Variables|Default|SetFoodIndex 0)
    (else
      (Variables|Default|SetFoodIndex (+ (Variables|Default|GetFoodIndex) 1)))))

(fn SelectFood
  (bind _output_get (Variables|Default|SetFoodTypes (Utilities|Select :Index (Variables|Default|GetFoodIndex) :Option%200 "NewEnumerator0" :Option%201 "NewEnumerator1" :Option%202 "NewEnumerator2")))
  (return _output_get))

(fn GetTextReference
  (bind _asfood_ui (Utilities|Casting|CastToFoodUI (UserInterface|GetWidget (Variables|Default|GetFoodSelectUI))))
  (Variables|Default|SetTextReference (Variables|/Game/Assets/UI/FoodUI.FoodUI_C|GetFoodText _asfood_ui)))

(fn RotateTowardsPlayer
  (params (Object%20To%20Rotate :type Scene%20Component%20Object%20Reference) (Start :type Vector%20%28by%20ref%29) (Target :type Vector%20%28by%20ref%29))
  (Transformation|SetWorldRotation Object%20To%20Rotate (Math|Rotator|Lerp(Rotator) (Math|Rotator|MakeRotator 0.0 0.0 (.yaw (Transformation|GetWorldRotation Object%20To%20Rotate))) (Math|Rotator|MakeRotator 0.0 0.0 (.yaw (Math|Rotator|FindLookatRotation Start Target))) 1.0 true) false false))

(fn GetSpawnLoc
  (bind _spawnpoint (Variables|Default|GetSpawnPoint))
  (bind _returnvalue (Transformation|GetWorldTransform _spawnpoint))
  (bind _output_get (Variables|Default|SetSpawnPos (Math|Transform|MakeTransform (.location _returnvalue) (.rotation _returnvalue) "0.250000,0.250000,0.250000")))
  (return _output_get))