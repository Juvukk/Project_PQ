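; PQ creature pawn with Passion, Quality, Pep and Peckish stats, capped at ten, that roams and eats food.
; Tick switches on an AiDo state to follow the player when leashed, wander randomly, or sphere-sense food and check it against its tastes.
; Completed follow or roam moves lower Peckish, and low Peckish while roaming triggers food search.
; Overlapping food destroys it, adjusts Pep by like or dislike, boosts Peckish and resumes roaming.
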(event EventBeginPlay
  (Variables|Stats|SetPeckish (Math|Random|RandomInteger 11)))

(event EventTick
  (params (DeltaSeconds :type Float%20%28single-precision%29))
  (CallFunction|LimitStatstoTen)
  (switch Utilities|FlowControl|Switch|SwitchonAIBehaviour (Variables|AIControl|GetAiDo)
    (:NewEnumerator0
      (bind _returnvalue (CallFunction|GetDistance))
      (CallFunction|CheckDistance _returnvalue _returnvalue _returnvalue)
      (AI|AIMoveTo self "0, 0, 0" (Game|GetPlayerCharacter 0) 1e+02 true
        (:then
          (Utilities|FlowControl|Delay 1e+01)
          (CallFunction|ChangePeckish -1 :!label _label))))
    (:NewEnumerator1
      (|CheckifHungry
        (:else
          (Utilities|FlowControl|Delay 1e+01 :!label _label_2)
          (bind _roamloc (CallFunction|GetRandomLocation :!label _label_3))
          (AI|AIMoveTo self _roamloc 0 1e+02 true
            (:then
              (goto _label))
            (:OnFail
              (goto _label_3))))))
    (:NewEnumerator2
      (if (Utilities|IsValid (Variables|AIControl|GetFoundFood))
        (AI|AIMoveTo self "0, 0, 0" (Variables|AIControl|GetFoundFood) 5.0 false)
        (else
          (bind _outactors (CallFunction|SenseFood))
          (if (>= (Utilities|Array|Length _outactors) 1)
            (bind _array_element (Utilities|Array|ForEachLoopwithBreak _outactors :!label _label_4)
              (:LoopBody
                (bind _nofoodfound (CallFunction|FindLikedFood _array_element _array_element))
                (if _nofoodfound
                  (goto _label_3)
                  (else
                    (goto _label_4 Break)))))
            (else
              (goto _label_2))))))))

(event Collision|EventActorBeginOverlap
  (params (OtherActor :type Actor%20Object%20Reference))
  (bind _asfood (Utilities|Casting|CastToFood OtherActor))
  (bind (_like_ _dislike) (CallFunction|DetermineLikeDislike _asfood))
  (bind _pepchange (CallFunction|ChangePepfromFood _like_ _dislike))
  (CallFunction|ChangePep _pepchange)
  (CallFunction|ChangePeckish 5)
  (Actor|DestroyActor OtherActor)
  (Variables|AIControl|SetAiDo "NewEnumerator1"))

(fn ConstructionScript)

(fn GetDistance
  (return (Math|Vector|Distance(Vector) (Transformation|GetActorLocation (Game|GetPlayerCharacter 0)) (Transformation|GetActorLocation))))

(fn CheckDistance
  (params (A :type Float%20%28double-precision%29) (PrevDist :type Float%20%28double-precision%29) (PrevDist2 :type Float%20%28double-precision%29))
  (if (> A (Variables|AIControl|GetPrevDist))
    (Variables|AIControl|SetPrevDist PrevDist2)
    (else
      (Variables|AIControl|SetPrevDist PrevDist))))

(fn GetRandomLocation
  (bind _output_get (LocalVariables|SetRandomLoc (Math|Vector|MakeVector (Math|Random|RandomFloatinRange 0.0 3.4e+03) (Math|Random|RandomFloatinRange 0.0 3.4e+03) (|GetZ))))
  (return _output_get))

(fn EatFood
  (params (FoodActor :type Actor%20Object%20Reference)))

(fn DetermineLikeDislike
  (params (FoodType :type Food%20Object%20Reference))
  (bind _like (Variables|Stats|GetLike))
  (bind _dislike (Variables|Stats|GetDislike))
  (bind _returnvalue (Utilities|Enum|Equal(Enum) _dislike (Variables|/Game/Blueprints/Food.Food_C|GetFoodType FoodType)))
  (bind _returnvalue_2 (Utilities|Enum|Equal(Enum) _like (Variables|/Game/Blueprints/Food.Food_C|GetFoodType FoodType)))
  (if _returnvalue_2
    (Development|PrintString "Like")
    (elif _returnvalue
      (Development|PrintString "Dislike")))
  (return _returnvalue_2 _returnvalue))

(fn ChangePepfromFood
  (params (Like :type Boolean) (Dislike :type Boolean))
  (if Like
    (LocalVariables|SetpepIncrease 2)
    (elif Dislike
      (LocalVariables|SetpepIncrease -2)
      (else
        (LocalVariables|SetpepIncrease 0))))
  (return (LocalVariables|GetpepIncrease)))

(fn ChangePep
  (params (Value :type Integer))
  (Variables|Stats|SetPep (+ (Variables|Stats|GetPep) Value)))

(fn ChangePeckish
  (params (ChangeAmount :type Integer))
  (Math|Integer|CompareInt (Variables|Stats|GetPeckish)
    (:>
      (Variables|Stats|SetPeckish (+ (Variables|Stats|GetPeckish) ChangeAmount)))))

(fn SenseFood
  (bind _returnvalue (Transformation|GetActorLocation))
  (Rendering|Debug|DrawDebugSphere _returnvalue 2.5e+02 12 "(R=0.192090,G=0.414062,B=0.000000,A=1.000000)" 0.0)
  (bind _outactors (Collision|SphereOverlapActors _returnvalue 2.5e+02 (Utilities|Array|MakeArray "ObjectTypeQuery8") "/Game/Blueprints/Food.Food_C"))
  (return _outactors))

(fn FindLikedFood
  (params (Object :type Object%20Object%20Reference) (FoundFood :type Actor%20Object%20Reference))
  (bind _asfood (Utilities|Casting|CastToFood Object))
  (bind _like_ (CallFunction|DetermineLikeDislike _asfood))
  (if _like_
    (LocalVariables|SetNothingFound false)
    (Variables|AIControl|SetFoundFood FoundFood :!label _label)
    (elif (Utilities|Enum|Equal(Enum) (Variables|Stats|GetNeutral) (Variables|/Game/Blueprints/Food.Food_C|GetFoodType _asfood))
      (goto _label)
      (else
        (LocalVariables|SetNothingFound true))))
  (return (LocalVariables|GetNothingFound)))

(fn LimitStatstoTen
  (Utilities|FlowControl|Sequence
    (:then_0
      (Math|Integer|CompareInt (Variables|Stats|GetPassion) 10
        (:>
          (Variables|Stats|SetPassion 10))))
    (:then_1
      (Math|Integer|CompareInt (Variables|Stats|GetQuality) 10
        (:>
          (Variables|Stats|SetQuality 10))))
    (:then_2
      (Math|Integer|CompareInt (Variables|Stats|GetPep) 10
        (:>
          (Variables|Stats|SetPep 10))))
    (:then_3
      (Math|Integer|CompareInt (Variables|Stats|GetPeckish) 10
        (:>
          (Variables|Stats|SetPeckish 10))))))