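; Animal is a short-lived projectile pickup that adds its PeckFill value to the Peckish stat of a Bp_PQ actor that overlaps it, then destroys itself.
; On BeginPlay, NewFunction0 launches it upward with a random horizontal speed along either local X or Y, chosen at random.
; A Delay driven from Tick destroys the actor after LifeTime if nothing collects it.
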(event EventBeginPlay
  (CallFunction|NewFunction0))

(event Collision|EventActorBeginOverlap
  (params (OtherActor :type Actor%20Object%20Reference))
  (bind _asbp_pq (Utilities|Casting|CastToBp_PQ OtherActor))
  (Variables|/Game/Blueprints/Bp_PQ.Bp_PQ_C|SetPeckish _asbp_pq (+ (Variables|Default|GetPeckFill) (Variables|/Game/Blueprints/Bp_PQ.Bp_PQ_C|GetPeckish _asbp_pq) 0))
  (Actor|DestroyActor))

(event EventTick
  (params (DeltaSeconds :type Float%20%28single-precision%29))
  (Utilities|FlowControl|Delay (Variables|Default|GetLifeTime))
  (Actor|DestroyActor))

(fn ConstructionScript)

(fn NewFunction0
  (if (Math|Random|RandomBool)
    (Game|Components|ProjectileMovement|SetVelocityinLocalSpace (Variables|Default|GetProjectileMovement) (Math|Vector|MakeVector (Math|Random|RandomFloatinRange -5e+02 5e+02) 0.0 5e+02))
    (else
      (Game|Components|ProjectileMovement|SetVelocityinLocalSpace (Variables|Default|GetProjectileMovement) (Math|Vector|MakeVector 0.0 (Math|Random|RandomFloatinRange -5e+02 5e+02) 5e+02)))))