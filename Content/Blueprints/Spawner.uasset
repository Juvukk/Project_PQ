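; Breeding station that spawns a child Bp_PQ when its button is hit, if both parents are valid and their combined Passion is high enough.
; Tick claims unleashed PQs in two collision volumes as Mum and Dad and stops their roaming.
; Children derive texture and colour from summed parent indices (random on overflow), serif or sans mesh from Pep, and random distinct likes.
; Dynamic material instances apply looks to existing and spawned PQs.
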(event OnComponentEndOverlap(FatherCol)
  (params (OverlappedComponent :type Primitive%20Component%20Object%20Reference) (OtherActor :type Actor%20Object%20Reference) (OtherComp :type Primitive%20Component%20Object%20Reference) (OtherBodyIndex :type Integer))
  (bind _asbp_pq (Utilities|Casting|CastToBp_PQ OtherActor))
  (bind _returnvalue (CallFunction|CheckifLeashed _asbp_pq))
  (if (not _returnvalue)
    (CallFunction|SetRoam _asbp_pq true)
    (Variables|Default|SetDad 0)))

(event OnComponentEndOverlap(MotherCol)
  (params (OverlappedComponent :type Primitive%20Component%20Object%20Reference) (OtherActor :type Actor%20Object%20Reference) (OtherComp :type Primitive%20Component%20Object%20Reference) (OtherBodyIndex :type Integer))
  (bind _asbp_pq (Utilities|Casting|CastToBp_PQ OtherActor))
  (bind _returnvalue (CallFunction|CheckifLeashed _asbp_pq))
  (if (not _returnvalue)
    (CallFunction|SetRoam _asbp_pq true)
    (Variables|Default|SetMum 0)))

(event Custom|SpawnChild
  (params (HitButton :type Static%20Mesh%20Component%20Object%20Reference))
  (bind _cylinder (Variables|Default|GetCylinder))
  (bind _returnvalue (Transformation|GetWorldLocation _cylinder))
  (if (== HitButton (Variables|Default|GetBp_Button))
    (Utilities|FlowControl|Sequence
      (:then_0
        (bind _isvalid (CallFunction|ValidateParent (Variables|Default|GetMum))))
      (:then_1
        (bind _isvalid_2 (CallFunction|ValidateParent (Variables|Default|GetDad))))
      (:then_2
        (if (and _isvalid _isvalid_2)
          (bind _ispassionate (CallFunction|DetermineParentPassion))
          (if _ispassionate
            (bind _returnvalue_2 (Game|SpawnActorfromClass "/Game/Blueprints/Bp_PQ.Bp_PQ_C" (Math|Transform|MakeTransform (Math|Vector|MakeVector (.x _returnvalue) (.y _returnvalue) 6e+01) "0, 0, 0" "1.000000,1.000000,1.000000") "Undefined" 0 0))
            (Variables|Default|SetChild _returnvalue_2)
            (CallFunction|SetChildPassonTex)
            (CallFunction|SetChildPassCol)
            (CallFunction|SetMaterial (Variables|Default|GetChild))
            (bind _isserif (CallFunction|DetermineSerif))
            (if _isserif
              (CallFunction|SetChildSerif (Variables|Default|GetAllSerif))
              (else
                (CallFunction|SetChildSerif (Variables|Default|GetAllSans))))
            (CallFunction|SetChildLikes (Variables|Default|GetChild))
            (CallFunction|ResetParentPassion)
            (else
              (Development|PrintString "ParentPassion not High Enough")))
          (else
            (Development|PrintString "Can't Spawn Parents Invalid")))))))

(event EventBeginPlay
  (bind _asbp_first_person_character (Utilities|Casting|CastToBP_FirstPersonCharacter (Game|GetPlayerCharacter 0)))
  (EventDispatchers|AssignButtonEvent _asbp_first_person_character (delegate Custom|SpawnChild))
  (bind _outactors (Actor|GetAllActorsOfClass "/Game/Blueprints/Bp_PQ.Bp_PQ_C"))
  (for _array_element _outactors
    (CallFunction|SetMaterial _array_element)))

(event EventTick
  (params (DeltaSeconds :type Float%20%28single-precision%29))
  (Utilities|FlowControl|Sequence
    (:then_0
      (bind _asbp_pq (Utilities|Casting|CastToBp_PQ (Utilities|Array|Get(acopy) (Collision|GetOverlappingActors (Variables|Default|GetFatherCol) "/Game/Blueprints/Bp_PQ.Bp_PQ_C" :!class /Script/Engine.PrimitiveComponent))))
      (bind _returnvalue (CallFunction|CheckifLeashed _asbp_pq))
      (if (not _returnvalue)
        (if (Actor|ActorHasTag _asbp_pq "PQ")
          (bind _output_get (Variables|Default|SetMum _asbp_pq))
          (CallFunction|SetRoam _output_get false))))
    (:then_1
      (bind _asbp_pq_2 (Utilities|Casting|CastToBp_PQ (Utilities|Array|Get(acopy) (Collision|GetOverlappingActors (Variables|Default|GetMotherCol) "/Game/Blueprints/Bp_PQ.Bp_PQ_C" :!class /Script/Engine.PrimitiveComponent))))
      (bind _returnvalue_2 (CallFunction|CheckifLeashed _asbp_pq_2))
      (if (not _returnvalue_2)
        (if (Actor|ActorHasTag _asbp_pq_2 "PQ")
          (bind _output_get_2 (Variables|Default|SetDad _asbp_pq_2))
          (CallFunction|SetRoam _output_get_2 false))))))

(fn ConstructionScript)

(fn SetChildPassonTex
  (bind _alltextures (Variables|Default|GetAllTextures))
  (bind _child (Variables|Default|GetChild))
  (bind _returnvalue (Utilities|Array|Length _alltextures))
  (if (> (+ (Variables|/Game/Blueprints/Bp_PQ.Bp_PQ_C|GetPassOnTex (Variables|Default|GetMum)) (Variables|/Game/Blueprints/Bp_PQ.Bp_PQ_C|GetPassOnTex (Variables|Default|GetDad))) _returnvalue)
    (Variables|/Game/Blueprints/Bp_PQ.Bp_PQ_C|SetPassOnTex _child (Math|Random|RandomIntegerinRange 0 _returnvalue))
    (else
      (Variables|/Game/Blueprints/Bp_PQ.Bp_PQ_C|SetPassOnTex _child (+ (Variables|/Game/Blueprints/Bp_PQ.Bp_PQ_C|GetPassOnTex (Variables|Default|GetMum)) (Variables|/Game/Blueprints/Bp_PQ.Bp_PQ_C|GetPassOnTex (Variables|Default|GetDad)))))))

(fn ValidateParent
  (params (ParentCollision :type Bp%20PQ%20Object%20Reference))
  (bind _returnvalue (Utilities|IsValid ParentCollision))
  (if _returnvalue
    (return ParentCollision _returnvalue)
    (else
      (Development|PrintString (Utilities|String|Append "Parent Invalid:" (Utilities|GetDisplayName ParentCollision))))))

(fn SetMaterial
  (params (ActorToSet :type Bp%20PQ%20Object%20Reference))
  (bind _pq_mesh (Variables|/Game/Blueprints/Bp_PQ.Bp_PQ_C|GetPQ_Mesh ActorToSet))
  (bind _returnvalue (Rendering|Material|CreateDynamicMaterialInstance _pq_mesh 0 "/Game/Assets/Materials/Master/Mat_PQMaster.Mat_PQMaster" "None" :!class /Script/Engine.PrimitiveComponent))
  (bind _output_get (Variables|Default|SetChildMaterialInstance _returnvalue))
  (Rendering|Material|SetTextureParameterValue _output_get "Tex" (Utilities|Array|Get(acopy) (Variables|Default|GetAllTextures) (Variables|/Game/Blueprints/Bp_PQ.Bp_PQ_C|GetPassOnTex ActorToSet)))
  (Rendering|Material|SetVectorParameterValue (Variables|Default|GetChildMaterialInstance) "Tint" (Utilities|Array|Get(acopy) (Variables|Default|GetAllColours) (Variables|/Game/Blueprints/Bp_PQ.Bp_PQ_C|GetPassOnCol ActorToSet)) :!class /Script/Engine.MaterialInstanceDynamic)
  (Rendering|Material|SetMaterial _pq_mesh 0 (Variables|Default|GetChildMaterialInstance)))

(fn SetChildPassCol
  (bind _child (Variables|Default|GetChild))
  (bind _allcolours (Variables|Default|GetAllColours))
  (bind _returnvalue (Utilities|Array|Length _allcolours))
  (if (> (+ (Variables|/Game/Blueprints/Bp_PQ.Bp_PQ_C|GetPassOnCol (Variables|Default|GetMum)) (Variables|/Game/Blueprints/Bp_PQ.Bp_PQ_C|GetPassOnCol (Variables|Default|GetDad))) _returnvalue)
    (Variables|/Game/Blueprints/Bp_PQ.Bp_PQ_C|SetPassOnCol _child (Math|Random|RandomIntegerinRange 0 _returnvalue))
    (else
      (Variables|/Game/Blueprints/Bp_PQ.Bp_PQ_C|SetPassOnCol _child (+ (Variables|/Game/Blueprints/Bp_PQ.Bp_PQ_C|GetPassOnCol (Variables|Default|GetMum)) (Variables|/Game/Blueprints/Bp_PQ.Bp_PQ_C|GetPassOnCol (Variables|Default|GetDad)))))))

(fn SetChildSerif
  (params (MeshList :type Array%20of%20Static%20Mesh%20Object%20References))
  (Components|StaticMesh|SetStaticMesh (Variables|/Game/Blueprints/Bp_PQ.Bp_PQ_C|GetPQ_Mesh (Variables|Default|GetChild)) (Utilities|Array|Get(acopy) MeshList (Math|Random|RandomIntegerinRange 0 (- (Utilities|Array|Length MeshList) 1)))))

(fn DetermineSerif
  (return (<= (|((MumPep+DadPep)/1.500000) (Math|Conversions|ToFloat(Integer) (Variables|/Game/Blueprints/Bp_PQ.Bp_PQ_C|GetPep (Variables|Default|GetMum))) (Math|Conversions|ToFloat(Integer) (Variables|/Game/Blueprints/Bp_PQ.Bp_PQ_C|GetPep (Variables|Default|GetDad)))) 5.0)))

(fn SetRoam
  (params (Parent :type Bp%20PQ%20Object%20Reference) (AllowRoam :type Boolean))
  (if (Utilities|IsValid Parent)
    (if AllowRoam
      (Variables|/Game/Blueprints/Bp_PQ.Bp_PQ_C|SetAiDo Parent "NewEnumerator1")
      (else
        (Variables|/Game/Blueprints/Bp_PQ.Bp_PQ_C|SetAiDo Parent "NewEnumerator3")))))

(fn SetChildLikes
  (params (Child :type Bp%20PQ%20Object%20Reference))
  (Utilities|FlowControl|Sequence
    (:then_0
      (bind _returnvalue (CallFunction|GetRandomLikes))
      (Variables|/Game/Blueprints/Bp_PQ.Bp_PQ_C|SetLike Child _returnvalue))
    (:then_1
      (bind _returnvalue_2 (CallFunction|GetRandomLikes :!label _label))
      (if (Utilities|Enum|Equal(Enum) _returnvalue_2 (Variables|/Game/Blueprints/Bp_PQ.Bp_PQ_C|GetLike Child))
        (goto _label)
        (else
          (Variables|/Game/Blueprints/Bp_PQ.Bp_PQ_C|SetDislike Child _returnvalue_2))))
    (:then_2
      (bind _returnvalue_3 (CallFunction|GetRandomLikes :!label _label_2))
      (if (Utilities|Enum|Equal(Enum) (Variables|/Game/Blueprints/Bp_PQ.Bp_PQ_C|GetLike Child) _returnvalue_3)
        (goto _label_2)
        (elif (Utilities|Enum|Equal(Enum) (Variables|/Game/Blueprints/Bp_PQ.Bp_PQ_C|GetDislike Child) _returnvalue_3)
          (goto _label_2)
          (else
            (Variables|/Game/Blueprints/Bp_PQ.Bp_PQ_C|SetNeutral Child _returnvalue_3)))))))

(fn GetRandomLikes
  (return (Utilities|Select :Index (Math|Random|RandomInteger 3) :Option%200 "NewEnumerator0" :Option%201 "NewEnumerator1" :Option%202 "NewEnumerator2")))

(fn ResetParentPassion
  (Variables|/Game/Blueprints/Bp_PQ.Bp_PQ_C|SetPassion (Variables|Default|GetMum) 0)
  (Variables|/Game/Blueprints/Bp_PQ.Bp_PQ_C|SetPassion (Variables|Default|GetDad) 0))

(fn DetermineParentPassion
  (return (>= (+ (Variables|/Game/Blueprints/Bp_PQ.Bp_PQ_C|GetPassion (Variables|Default|GetMum)) (Variables|/Game/Blueprints/Bp_PQ.Bp_PQ_C|GetPassion (Variables|Default|GetDad))) 10)))

(fn CheckifLeashed
  (params (Parent :type Bp%20PQ%20Object%20Reference))
  (if (Utilities|IsValid Parent)
    (return (Utilities|Enum|Equal(Enum) (Variables|/Game/Blueprints/Bp_PQ.Bp_PQ_C|GetAiDo Parent) "NewEnumerator0"))))